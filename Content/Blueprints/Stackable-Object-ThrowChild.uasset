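; Throwable child variant of a stackable object that launches its Body toward the player turtle character.
; BeginPlay picks a random launch multiplier without running the parent BeginPlay.
; Throw computes a suggested projectile arc to the turtle, halves its horizontal velocity, substitutes a fixed upward component, and applies the scaled result as a mass-dependent impulse.
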(event EventBeginPlay
  (Variables|Default|SetLaunchMultiplier (Math|Random|RandomFloatinRange 2.5e+02 3e+02)))

(event Collision|EventActorBeginOverlap
  (params (OtherActor :type Actor%20Object%20Reference))
  (|CallParentFunction OtherActor) ; This node is disabled and will not be called.\nDrag off pins to build functionality.
)

(event EventTick
  (params (DeltaSeconds :type Float%20%28single-precision%29))
  (|CallParentFunction DeltaSeconds) ; This node is disabled and will not be called.\nDrag off pins to build functionality.
)

(fn ConstructionScript
  (|CallParentFunction))

(fn Throw
  (bind _returnvalue (Actor|GetActorOfClass "/Game/Blueprints/Player/PlayerTurtleCharacter.PlayerTurtleCharacter_C"))
  (bind _outlaunchvelocity (Game|SuggestProjectileVelocityCustomArc (Transformation|GetActorLocation) (Transformation|GetActorLocation _returnvalue) 0.0 0.5))
  (Physics|AddImpulse (Variables|Default|GetBody) (* (Math|Vector|MakeVector (/ (.X (Math|Vector|BreakVector _outlaunchvelocity)) 2.0) (/ (.Y (Math|Vector|BreakVector _outlaunchvelocity)) 2.0) 1e+03) (Variables|Default|GetLaunchMultiplier)) "None" false))