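; Test stackable object that flies toward where the player turtle stood at spawn, apparently prototyping an arcing throw.
; BeginPlay samples the PlayerTurtleCharacterOLD location once and sets a target height above it.
; Tick lowers that target by a fixed, frame-rate-dependent step and chases it with constant-speed interpolation, without sweep.
; Any actor overlap destroys the object.
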(event EventBeginPlay
  (Variables|Default|SetCurrentLocation (Transformation|GetActorLocation))
  (bind _returnvalue (Actor|GetActorOfClass "/Game/Blueprints/Player/PlayerTurtleCharacter-OLD.PlayerTurtleCharacter-OLD_C"))
  (bind _output_get (Variables|Default|SetTargetLocation (Transformation|GetActorLocation _returnvalue)))
  (Variables|Default|SetTargetZValue (.Z (Math|Vector|BreakVector _output_get)))
  (bind _output_get_2 (Variables|Default|SetZTopLocation (+ (.Z (Math|Vector|BreakVector _output_get)) 5e+02)))
  (Variables|Default|SetCurrZTop _output_get_2))

(event EventTick
  (params (DeltaSeconds :type Float%20%28single-precision%29))
  (Actor|GetActorOfClass (Utilities|GetClass (stale Collision|EventActorBeginOverlap OtherActor)))
  (Variables|Default|SetFrameTime DeltaSeconds)
  (bind _output_get (Variables|Default|SetTargetLocation (Math|Vector|MakeVector (.X (Math|Vector|BreakVector (Variables|Default|GetTargetLocation))) (.Y (Math|Vector|BreakVector (Variables|Default|GetTargetLocation))) (- (Variables|Default|GetCurrZTop) 5e+01))))
  (Variables|Default|SetCurrZTop (- (Variables|Default|GetCurrZTop) 5e+01))
  (bind _output_get_2 (Variables|Default|SetCurrentLocation (Math|Interpolation|VInterptoConstant (Variables|Default|GetCurrentLocation) _output_get (Variables|Default|GetFrameTime) 1e+03)))
  (Transformation|SetActorLocation _output_get_2 false false))

(event Collision|EventActorBeginOverlap
  (params (OtherActor :type Actor%20Object%20Reference))
  (Actor|DestroyActor))

(fn ConstructionScript)