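; Obsolete player prototype of a teetering item stack, filled through fixed slots Item0 to Item6.
; BeginPlay selects the first slot and places the collision-disabled StackDetector there.
; AddItemToStack attaches the item, but always repositions it above Base and links it to Item1 through PhysicsConstraint0, whichever slot is current.
; MoveStackUp advances the slot via nested branches, doubles its world location and clears CanStack upon reaching the last.
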(event EventBeginPlay
  (CallFunction|InitializeStack))

(fn ConstructionScript)

(fn InitializeStack
  (bind _stackdetector (Variables|Default|GetStackDetector))
  (Utilities|FlowControl|Sequence
    (:then_0
      (Variables|Default|SetCurrentItemSlot (Variables|ItemSlot|GetItem0)))
    (:then_1
      ;[1 0.3008 0.2809] Setup Stack Detector
      (Transformation|SetRelativeLocation _stackdetector (Variables|/Script/Engine.SceneComponent|GetRelativeLocation (Variables|Default|GetCurrentItemSlot)) false false)
      (Collision|SetCollisionEnabled _stackdetector "NoCollision"))))

(fn AddItemtoStack
  (params (NewItem :type Stackable%20Object%20Base%20Object%20Reference))
  (bind _output_get (Variables|Default|SetNewStackItem NewItem))
  (Utilities|IsValid _output_get
    (:Is%20Valid
      (Utilities|FlowControl|Sequence
        (:then_0
          ;[1 1 1] Change New Item's Collision
          (Collision|SetCollisionEnabled (Variables|/Game/Blueprints/StackableObjects/Testing/StackableObjectBase.StackableObjectBase_C|GetCylinder (Variables|Default|GetNewStackItem)) (Collision|GetCollisionEnabled (Variables|Default|GetCurrentItemSlot))))
        (:then_1
          ;[1 1 1] Attach Object to the item slot
          (Transformation|AttachComponentToComponent (Variables|Default|GetNewStackItem) (Variables|Default|GetCurrentItemSlot) "None" "SnapToTarget" "KeepRelative" "KeepRelative" false))
        (:then_2
          (if true
            ;[1 1 1] Attached to Base
            (Transformation|SetActorLocation (Variables|Default|GetNewStackItem) (+ (Transformation|GetWorldLocation (Variables|Default|GetBase)) (Math|Vector|MakeVector 0.0 0.0 (/ (.SphereRadius (Collision|GetComponentBounds (Variables|/Game/Blueprints/StackableObjects/Testing/StackableObjectBase.StackableObjectBase_C|GetCylinder (Variables|Default|GetNewStackItem)))) 1.5))) false false)))
        (:then_3
          (Transformation|SetWorldLocation (Variables|Default|GetPhysicsConstraint0) (Transformation|GetWorldLocation (Variables|/Game/Blueprints/StackableObjects/Testing/StackableObjectBase.StackableObjectBase_C|GetTopPoint (Variables|Default|GetNewStackItem))) false false)
          (Class|PhysicsConstraintComponent|SetConstrainedComponents (Variables|Default|GetPhysicsConstraint0) (Variables|/Game/Blueprints/StackableObjects/Testing/StackableObjectBase.StackableObjectBase_C|GetCylinder (Variables|Default|GetNewStackItem)) "None" (Variables|ItemSlot|GetItem1) "None"))
        (:then_4
          (CallFunction|MoveStackUp))))))

(fn MoveStackUp
  (bind _currentitemslot (Variables|Default|GetCurrentItemSlot))
  (CallFunction|SetNextSlot)
  (Transformation|SetWorldLocation _currentitemslot (* (Transformation|GetWorldLocation _currentitemslot) 2.0) false false))

(fn SetNextSlot
  (if (== (Variables|Default|GetCurrentItemSlot) (Variables|ItemSlot|GetItem0))
    (Variables|Default|SetCurrentItemSlot (Variables|ItemSlot|GetItem1))
    (elif (== (Variables|Default|GetCurrentItemSlot) (Variables|ItemSlot|GetItem1))
      (Variables|Default|SetCurrentItemSlot (Variables|ItemSlot|GetItem2))
      (elif (== (Variables|Default|GetCurrentItemSlot) (Variables|ItemSlot|GetItem2))
        (Variables|Default|SetCurrentItemSlot (Variables|ItemSlot|GetItem3))
        (elif (== (Variables|Default|GetCurrentItemSlot) (Variables|ItemSlot|GetItem3))
          (Variables|Default|SetCurrentItemSlot (Variables|ItemSlot|GetItem4))
          (elif (== (Variables|Default|GetCurrentItemSlot) (Variables|ItemSlot|GetItem4))
            (Variables|Default|SetCurrentItemSlot (Variables|ItemSlot|GetItem5))
            (elif (== (Variables|Default|GetCurrentItemSlot) (Variables|ItemSlot|GetItem5))
              (Variables|Default|SetCurrentItemSlot (Variables|ItemSlot|GetItem6))
              (Variables|Default|SetCanStack false))))))))