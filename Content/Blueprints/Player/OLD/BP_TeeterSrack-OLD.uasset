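; An older player-side item stack Blueprint with seven placeholder slots, apparently for showing picked-up items as a stack.
; On BeginPlay, InitializeStack builds a map keyed by the placeholder components, with bools meant to track which slots are filled.
; It then loops over the keys to set each placeholder's visibility, intended to hide them at start.
; Pickup and next-free-slot logic are described in a comment but not implemented here.
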(event EventBeginPlay
  (CallFunction|InitializeStack))

(fn ConstructionScript)

(fn InitializeStack
  ;[1 0.6141 0.3474] Make map items with bools intialized to false
  ; *When an Item is picked up we'll be able to check though the index of the map to see what is the next slot to place the new item*
  (bind _output_get (Variables|Default|SetStackItems (Utilities|Map|MakeMap (Variables|Default|GetItem0) false (Variables|Default|GetItem1) false (Variables|Default|GetItem2) false (Variables|Default|GetItem3) false (Variables|Default|GetItem4) false (Variables|Default|GetItem5) false (Variables|Default|GetItem6) false)))
  ;[1 1 1] Make the placeholder items invisible on start
  (bind _keys (Utilities|Map|Keys _output_get))
  (for _array_element _keys
    (Rendering|SetVisibility _array_element (LocalVariables|GetTemp) false)))