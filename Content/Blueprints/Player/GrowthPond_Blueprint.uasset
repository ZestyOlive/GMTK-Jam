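; Growth pond actor that marks when the player's turtle character is inside its overlap area.
; On begin and end overlap, it checks that the other actor is a child of the evolving test turtle class, casts it, and sets or clears that turtle's IsInGrowthPond flag.
; Debug prints report overlaps, failed casts and non-turtle class names; any growth logic is not in this Blueprint.
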(event EventBeginPlay)

(event Collision|EventActorBeginOverlap
  (params (OtherActor :type Actor%20Object%20Reference))
  (bind _returnvalue (Utilities|GetClass OtherActor))
  (Development|PrintString "object is overlapping")
  (if (Utilities|ClassIsChildOf _returnvalue "/Game/Blueprints/Player/TestingTurtle-EvolvingTesting.TestingTurtle-EvolvingTesting_C")
    (bind _astesting_turtle__evolving_testing (Utilities|Casting|CastToTestingTurtle-EvolvingTesting OtherActor)
      (:then
        (Variables|/Game/Blueprints/Player/TestingTurtle-EvolvingTesting.TestingTurtle-EvolvingTesting_C|SetIsInGrowthPond _astesting_turtle__evolving_testing true)
        (Development|PrintString "in growth pond value changed"))
      (:CastFailed
        (Development|PrintString "cast failed")))
    (else
      (Development|PrintString "overlap object is not child of player turtle char")
      (Development|PrintString (Utilities|GetClassDisplayName _returnvalue)))))

(event EventTick
  (params (DeltaSeconds :type Float%20%28single-precision%29)))

(event Collision|EventActorEndOverlap
  (params (OtherActor :type Actor%20Object%20Reference))
  (if (Utilities|ClassIsChildOf (Utilities|GetClass OtherActor) "/Game/Blueprints/Player/TestingTurtle-EvolvingTesting.TestingTurtle-EvolvingTesting_C")
    (bind _astesting_turtle__evolving_testing (Utilities|Casting|CastToTestingTurtle-EvolvingTesting OtherActor))
    (Variables|/Game/Blueprints/Player/TestingTurtle-EvolvingTesting.TestingTurtle-EvolvingTesting_C|SetIsInGrowthPond _astesting_turtle__evolving_testing false)))

(fn ConstructionScript)